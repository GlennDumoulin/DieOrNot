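; GC_HasBullet is a gameplay cue that shows a debuff effect on a player character while the "has bullet" cue is active.
; On activation, if the character is alive, it points the DebuffSystem Niagara effect's skeletal mesh parameter at the character's mesh and activates it.
; It also plays a received-bullet force feedback effect through that character's player controller.
; Removing the cue deactivates the Niagara effect.
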(fn `OnActive`
  (params (MyTarget :type "Actor Object Reference") (Parameters :type "GameplayCueParameters Structure (by ref)"))
  (returns (ReturnValue :type Boolean))
  (bind _debuffsystem (`self.DebuffSystem`))
  (bind _asdonplayer_character (cast `DONPlayerCharacter` MyTarget))
  (if (`DONPlayerCharacter.bAlive` _asdonplayer_character)
    (`NiagaraFunctionLibrary.OverrideSystemUserVariableSkeletalMeshComponent` _debuffsystem "SkeletalMesh" (`Character.Mesh` _asdonplayer_character))
    (`ActorComponent.Activate` _debuffsystem true)
    (`PlayerController.K2_ClientPlayForceFeedback` (cast `PlayerController` (`Pawn.GetController` _asdonplayer_character) :!pure true) "/Game/Blueprints/HapticFeedbacks/FFE_ReceivedBullet.FFE_ReceivedBullet" "None" false true false)
    (return false)
    (else
      (return false))))

(fn `OnRemove`
  (params (MyTarget :type "Actor Object Reference") (Parameters :type "GameplayCueParameters Structure (by ref)"))
  (returns (ReturnValue :type Boolean))
  (`ActorComponent.Deactivate` (`self.DebuffSystem`))
  (return false))

(fn `UserConstructionScript`)