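; Gameplay cue for collecting a parry pickup, giving the player character visual, audio and haptic feedback.
; When the cue becomes active on a DON player character, it spawns a collect Niagara effect attached slightly below the root.
; If the character is alive, it also plays a quiet pickup sound with concurrency settings and sends controller force feedback that ignores time dilation.
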(fn `K2_HandleGameplayCue`
  (params (MyTarget :type "Actor Object Reference") (EventType :type "EGameplayCueEvent Enum" :default "OnActive") (Parameters :type "GameplayCueParameters Structure (by ref)"))
  (bind _rootcomponent (`Actor.RootComponent` MyTarget))
  (if (`|EnumEquality` EventType "OnActive")
    (bind _asdonplayer_character (cast `DONPlayerCharacter` MyTarget)
      (:`then`
        (`NiagaraFunctionLibrary.SpawnSystemAttached` "/Game/RFX/Systems/NS_PickUp_Collect.NS_PickUp_Collect" _rootcomponent "None" (0.0 0.0 -50.0) (struct) "SnapToTarget" true)
        (if (`DONPlayerCharacter.bAlive` _asdonplayer_character)
          (`GameplayStatics.PlaySoundAtLocation` _rootcomponent "/Game/SFX/Game/SW_PickupPickup.SW_PickupPickup" (`Actor.K2_GetActorLocation` MyTarget) (struct) 0.2 1.0 0.0 null "/Game/SFX/SoundClasses/SoundConcurrency.SoundConcurrency" (`GameplayStatics.GetPlayerCharacter` MyTarget) null)
          (`PlayerController.K2_ClientPlayForceFeedback` (cast `PlayerController` (`Pawn.GetController` _asdonplayer_character) :!pure true) "/Game/Blueprints/HapticFeedbacks/FFE_ParryPickup.FFE_ParryPickup" "None" false true false))
        (return))
      (:`CastFailed`
        _)))
  (return))