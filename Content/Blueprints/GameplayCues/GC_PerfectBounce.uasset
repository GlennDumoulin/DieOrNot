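; Gameplay cue for a perfect bounce on the DON player character, playing one-shot audio, visual and haptic feedback.
; OnExecute plays a sound and spawns a Niagara effect at the cue location, oriented along the forward vector of the source bullet.
; It shakes player 0's camera in proportion to bullet speed and sends force feedback to the character's controller, ignoring time dilation.
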(fn `OnExecute`
  (params (MyTarget :type "Actor Object Reference") (Parameters :type "GameplayCueParameters Structure (by ref)"))
  (returns (ReturnValue :type Boolean))
  (bind (_normalizedmagnitude _rawmagnitude _effectcontext _matchedtagname _originaltag _aggregatedsourcetags _aggregatedtargettags _location _normal _instigator _effectcauser _sourceobject) (`AbilitySystemBlueprintLibrary.BreakGameplayCueParameters` Parameters))
  (bind _asdonbullet (cast `DONBullet` _sourceobject :!pure true))
  (bind _asdonplayer_character (cast `DONPlayerCharacter` MyTarget)
    (:`then`
      (`GameplayStatics.PlaySoundAtLocation` MyTarget "/Game/SFX/Game/SW_PerfectBounce.SW_PerfectBounce" _location (struct) 1.0 1.0 0.0 null null null null)
      (`PlayerController.ClientStartCameraShake` :`self` (`GameplayStatics.GetPlayerController` null) :`Shake` "/Game/Blueprints/CameraShakes/BP_DefaultShake.BP_DefaultShake_C" :`Scale` (/ (`KismetMathLibrary.VSize` (`Actor.GetVelocity` _asdonbullet)) 1000.0))
      (`NiagaraFunctionLibrary.SpawnSystemAtLocation` MyTarget "/Game/RFX/Systems/NS_PerfectBounce.NS_PerfectBounce" _location (`KismetMathLibrary.Conv_VectorToRotator` (`Actor.GetActorForwardVector` _asdonbullet)))
      (`PlayerController.K2_ClientPlayForceFeedback` (cast `PlayerController` (`Pawn.GetController` _asdonplayer_character) :!pure true) "/Game/Blueprints/HapticFeedbacks/FFE_PerfectBounce.FFE_PerfectBounce" "None" false true false))
    (:`CastFailed`
      _))
  (return (`parent.OnExecute` MyTarget Parameters)))