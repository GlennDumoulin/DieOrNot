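; Gameplay Cue notify that plays jump feedback, a visual effect and a sound, for the player character.
; When executed on a DONPlayerCharacter target, it spawns the NS_Jump system attached to the character's root and plays SW_Jump at the target's location.
; It then hands off to the parent OnExecute for any target.
; An older version of the same effects remains in the EventGraph but never runs.
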(fn `OnExecute`
  (params (MyTarget :type "Actor Object Reference") (Parameters :type "GameplayCueParameters Structure (by ref)"))
  (returns (ReturnValue :type Boolean))
  (bind _asdonplayer_character (cast `DONPlayerCharacter` MyTarget)
    (:`then`
      (bind _returnvalue (`NiagaraFunctionLibrary.SpawnSystemAttached` "/Game/RFX/Systems/NS_Jump.NS_Jump" (`Actor.RootComponent` _asdonplayer_character) "None" (0.0 0.0 0.0) (struct) "KeepRelativeOffset" true))
      (`GameplayStatics.PlaySoundAtLocation` _returnvalue "/Game/SFX/Game/SW_Jump.SW_Jump" (`Actor.K2_GetActorLocation` MyTarget) (struct) 1.0 1.0 0.0 null null null null))
    (:`CastFailed`
      _))
  (return (`parent.OnExecute` MyTarget Parameters)))