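; Gameplay cue for a flash effect on the player character's bullets, going by its name tied to a bullet speed effect.
; OnActive loops over the target DONPlayerCharacter's Bullets, snapping the one Flash component to each root and activating it.
; Because that single component is re-attached each iteration, it ends up on the last bullet only.
; OnRemove deactivates Flash and prints a leftover "Hello" debug string.
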(fn `OnActive`
  (params (MyTarget :type "Actor Object Reference") (Parameters :type "GameplayCueParameters Structure (by ref)"))
  (returns (ReturnValue :type Boolean))
  (bind _flash (`self.Flash`))
  (for _array_element (`DONPlayerCharacter.Bullets` (cast `DONPlayerCharacter` MyTarget :!pure true))
    (`SceneComponent.K2_AttachToComponent` _flash (`Actor.RootComponent` _array_element) "None" "SnapToTarget" "SnapToTarget" "KeepRelative" true)
    (`ActorComponent.Activate` _flash true))
  (return true))

(fn `OnRemove`
  (params (MyTarget :type "Actor Object Reference") (Parameters :type "GameplayCueParameters Structure (by ref)"))
  (returns (ReturnValue :type Boolean))
  (`ActorComponent.Deactivate` (`self.Flash`))
  (`KismetSystemLibrary.PrintString` MyTarget)
  (return true))

(fn `UserConstructionScript`)