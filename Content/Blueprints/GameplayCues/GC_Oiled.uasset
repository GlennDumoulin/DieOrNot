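; Gameplay cue for the oiled status effect, giving feedback when a player character is hit by it.
; On activation it plays force feedback on the owning controller and attaches an oil malus Niagara system to the mesh, passing a fixed duration before activating it.
; On removal it clears the mesh overlay material, though the node that would apply the oil overlay is disconnected.
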(fn `OnActive`
  (params (MyTarget :type "Actor Object Reference") (Parameters :type "GameplayCueParameters Structure (by ref)"))
  (returns (ReturnValue :type Boolean))
  (bind _asdonplayer_character (cast `DONPlayerCharacter` MyTarget)
    (:`then`
      (`PlayerController.K2_ClientPlayForceFeedback` (cast `PlayerController` (`Pawn.GetController` _asdonplayer_character) :!pure true) "/Game/Blueprints/HapticFeedbacks/FFE_Oiled.FFE_Oiled" "None" false true false)
      (bind _returnvalue (`NiagaraFunctionLibrary.SpawnSystemAttached` "/Game/RFX/Systems/NS_oilMalus.NS_oilMalus" (`Character.Mesh` _asdonplayer_character) "None" (0.0 0.0 0.0) (struct) "KeepRelativeOffset" true false))
      (`NiagaraComponent.SetVariableFloat` _returnvalue "oil_malus_duration" 4.0)
      (`ActorComponent.Activate` _returnvalue true)
      (return false))
    (:`CastFailed`
      (return false))))

(fn `OnRemove`
  (params (MyTarget :type "Actor Object Reference") (Parameters :type "GameplayCueParameters Structure (by ref)"))
  (returns (ReturnValue :type Boolean))
  (bind _ascharacter (cast `Character` MyTarget))
  (`MeshComponent.SetOverlayMaterial` (`Character.Mesh` _ascharacter) null)
  (return false))

(fn `UserConstructionScript`)