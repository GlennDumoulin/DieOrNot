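; Gameplay cue that plays the feedback for a DON player character's death.
; On execute, it spawns a BP_PlayerDeathFracture actor at the character's transform, passing it the player, the cue location and the causing bullet.
; It also plays a death sound at that location and sends death force feedback to the player's controller, ignoring time dilation.
; Other targets go straight to the parent implementation.
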(fn `OnExecute`
  (params (MyTarget :type "Actor Object Reference") (Parameters :type "GameplayCueParameters Structure (by ref)"))
  (returns (ReturnValue :type Boolean))
  (bind (_normalizedmagnitude _rawmagnitude _effectcontext _matchedtagname _originaltag _aggregatedsourcetags _aggregatedtargettags _location _normal _instigator _effectcauser) (`AbilitySystemBlueprintLibrary.BreakGameplayCueParameters` Parameters))
  (bind _asdonplayer_character (cast `DONPlayerCharacter` MyTarget)
    (:`then`
      (`|SpawnActorFromClass` MyTarget "/Game/Blueprints/Gameplay/Effects/BP_PlayerDeathFracture.BP_PlayerDeathFracture_C" (`Actor.GetTransform` MyTarget) "Undefined" "OverrideRootScale" null _asdonplayer_character _location (cast `DONBullet` _effectcauser :!pure true) null)
      (`GameplayStatics.PlaySoundAtLocation` MyTarget "/Game/SFX/Game/SC_DeathCue.SC_DeathCue" _location (struct) 1.0 1.0 0.0 null null null null)
      (`PlayerController.K2_ClientPlayForceFeedback` (cast `PlayerController` (`Pawn.GetController` _asdonplayer_character) :!pure true) "/Game/Blueprints/HapticFeedbacks/FFE_PlayerDeath.FFE_PlayerDeath" "None" false true false)
      (return (`parent.OnExecute` MyTarget Parameters)))
    (:`CastFailed`
      (return (`parent.OnExecute` MyTarget Parameters)))))