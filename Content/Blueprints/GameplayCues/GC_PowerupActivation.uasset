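; Gameplay cue that plays powerup activation feedback when executed on a DONPlayerCharacter.
; It attaches a particle system to the target's root component and plays a sound at the character's location.
; Camera shake goes to player controller 0, while force feedback, ignoring time dilation, goes to the character's own controller.
; It then returns the parent OnExecute result.
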(fn `OnExecute`
  (params (MyTarget :type "Actor Object Reference") (Parameters :type "GameplayCueParameters Structure (by ref)"))
  (returns (ReturnValue :type Boolean))
  (bind _asdonplayer_character (cast `DONPlayerCharacter` MyTarget)
    (:`then`
      (`NiagaraFunctionLibrary.SpawnSystemAttached` "/Game/RFX/Systems/NS_PowerupActivation.NS_PowerupActivation" (`Actor.RootComponent` MyTarget) "None" (0.0 0.0 0.0) (struct) "SnapToTarget" true)
      (`GameplayStatics.PlaySoundAtLocation` MyTarget "/Game/SFX/Game/SW_PowerupActivate.SW_PowerupActivate" (`Actor.K2_GetActorLocation` _asdonplayer_character) (struct) 1.0 1.0 0.0 null null null null)
      (`PlayerController.ClientStartCameraShake` :`self` (`GameplayStatics.GetPlayerController` _asdonplayer_character) :`Shake` "/Game/Blueprints/CameraShakes/BP_PowerupActivation.BP_PowerupActivation_C")
      (`PlayerController.K2_ClientPlayForceFeedback` (cast `PlayerController` (`Pawn.GetController` _asdonplayer_character) :!pure true) "/Game/Blueprints/HapticFeedbacks/FFE_PowerupActivation.FFE_PowerupActivation" "None" false true false))
    (:`CastFailed`
      _))
  (return (`parent.OnExecute` MyTarget Parameters)))