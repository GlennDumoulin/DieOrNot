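; GC_Shoot is a gameplay cue that plays shot feedback when a DONPlayerCharacter fires.
; On execute, it spawns the NS_Shooting effect at the character's location, rotated to match the last entry in its Bullets array.
; It also plays the gunshot sound there and sends shoot force feedback to the character's player controller, ignoring time dilation.
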(fn `OnExecute`
  (params (MyTarget :type "Actor Object Reference") (Parameters :type "GameplayCueParameters Structure (by ref)"))
  (returns (ReturnValue :type Boolean))
  (bind _asdonplayer_character (cast `DONPlayerCharacter` MyTarget)
    (:`then`
      (bind _returnvalue (`Actor.K2_GetActorLocation` _asdonplayer_character))
      (bind _bullets (`DONPlayerCharacter.Bullets` _asdonplayer_character))
      (bind _returnvalue_2 (`NiagaraFunctionLibrary.SpawnSystemAtLocation` MyTarget "/Game/RFX/Systems/NS_Shooting.NS_Shooting" _returnvalue (`Actor.K2_GetActorRotation` (`|GetArrayItem` _bullets (`KismetArrayLibrary.Array_LastIndex` _bullets)))))
      (`GameplayStatics.PlaySoundAtLocation` _returnvalue_2 "/Game/SFX/Game/SC_GunShot_Cue.SC_GunShot_Cue" _returnvalue (struct) 0.8 1.0 0.0 null null null null)
      (`PlayerController.K2_ClientPlayForceFeedback` (cast `PlayerController` (`Pawn.GetController` _asdonplayer_character) :!pure true) "/Game/Blueprints/HapticFeedbacks/FFE_Shoot.FFE_Shoot" "None" false true false))
    (:`CastFailed`
      _))
  (return (`parent.OnExecute` MyTarget Parameters)))