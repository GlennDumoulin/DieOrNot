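; GC_FlashBullet is a gameplay cue that puts a flash effect on the bullets of a DON player character.
; When the cue becomes active, it loops over the target character's Bullets and attaches an auto-destroying NS_FlashBullet Niagara system to each bullet's root.
; Each system spawns inactive, receives the player's color as its Color parameter, then activates.
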(fn `OnActive`
  (params (MyTarget :type "Actor Object Reference") (Parameters :type "GameplayCueParameters Structure (by ref)"))
  (returns (ReturnValue :type Boolean))
  (bind _asdonplayer_character (cast `DONPlayerCharacter` MyTarget :!pure true))
  (for _array_element (`DONPlayerCharacter.Bullets` _asdonplayer_character)
    (bind _returnvalue (`NiagaraFunctionLibrary.SpawnSystemAttached` "/Game/RFX/Systems/NS_FlashBullet.NS_FlashBullet" (`Actor.RootComponent` _array_element) "None" (0.0 0.0 0.0) (struct) "SnapToTargetIncludingScale" true false))
    (`NiagaraComponent.SetVariableLinearColor` _returnvalue "Color" (`DONPlayerCharacter.GetPlayerColor` _asdonplayer_character))
    (`ActorComponent.Activate` _returnvalue true))
  (return (`parent.OnActive` MyTarget Parameters)))