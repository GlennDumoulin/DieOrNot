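; GA_AbilityShoot is a Gameplay Ability that makes the player character fire a shot with heavy recoil.
; Activation halts movement, applies GE_Shoot to the owner and plays the AM_Shoot montage.
; The montage notify calls Shoot, launches the character opposite the returned actor's forward vector and executes the shoot GameplayCue.
; The ability ends when the montage completes, blends out or is interrupted.
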(event `self.K2_ActivateAbility`
  (bind _returnvalue (`self.MakeOutgoingGameplayEffectSpec` "/Game/Blueprints/Abilities/GE_Shoot.GE_Shoot_C"))
  (bind (_returnvalue_owneractor _returnvalue_avataractor _returnvalue_playercontroller _returnvalue_abilitysystemcomponent _returnvalue_skeletalmeshcomponent _returnvalue_animinstance _returnvalue_movementcomponent) (break `GameplayAbilityActorInfo` (`self.GetActorInfo`)))
  (`AbilitySystemBlueprintLibrary.SetDuration` _returnvalue 2.0)
  (`MovementComponent.StopMovementImmediately` _returnvalue_movementcomponent)
  (`self.K2_ApplyGameplayEffectSpecToOwner` _returnvalue)
  (`|PlayMontage` _returnvalue_skeletalmeshcomponent "/Game/Assets/Character/Animations/AM_Shoot.AM_Shoot"
    (:`OnCompleted`
      (`self.K2_EndAbility` :!label _label))
    (:`OnBlendOut`
      (goto _label))
    (:`OnInterrupted`
      (goto _label))
    (:`OnNotifyBegin`
      (bind _returnvalue_2 (`self.Shoot`))
      (`Character.LaunchCharacter` (cast `DONPlayerCharacter` _returnvalue_owneractor :!pure true) (* (`Actor.GetActorForwardVector` _returnvalue_2) -8000.0) true true)
      (`self.K2_ExecuteGameplayCue` (struct :`TagName` "GameplayCue.Player.Shoot")))))