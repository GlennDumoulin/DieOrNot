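; Gameplay ability that opens a timed window for a perfect bullet bounce.
; It races a delay of half an owner attribute against a wait for the HasBounced tag.
; A bounce applies GE_PerfectBounce, or its Scale variant with the large-bullet tag, commits the success cooldown and cues the first bullet.
; A timeout commits the fail cooldown and plays the fail cue on a random bullet.
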(event `self.K2_ActivateAbility`
  (bind _returnvalue (`self.GetAbilitySystemComponentFromActorInfo`))
  (bind _output (`|GetArrayItem` (`DONPlayerCharacter.Bullets` (cast `DONPlayerCharacter` (`self.GetOwningActorFromActorInfo`) :!pure true))))
  (bind _asynctaskproxy (`AbilityTask_WaitDelay.WaitDelay` (* (`.ReturnValue` (`AbilitySystemBlueprintLibrary.GetFloatAttribute` (`self.GetOwningActorFromActorInfo`) (struct :`AttributeName` "ReactionTime" :`Attribute` "/Script/DON.PlayerAttributeSet:ReactionTime" :`AttributeOwner` "/Script/CoreUObject.Class'\"/Script/DON.PlayerAttributeSet\"'"))) 0.5))
    (:`then`
      (set `self.WaitTask` _asynctaskproxy)
      (bind _asynctaskproxy_2 (`AbilityTask_WaitGameplayTagAdded.WaitGameplayTagAdd` (struct :`TagName` "Event.Bullet.HasBounced") null true)
        (:`then`
          (set `self.BounceTask` _asynctaskproxy_2))
        (:`Added`
          (`GameplayTask.EndTask` (`self.WaitTask`))
          (`AbilitySystemComponent.BP_ApplyGameplayEffectToSelf` :`self` _returnvalue :`GameplayEffectClass` (select `bool` (`GameplayTagAssetInterface.HasMatchingGameplayTag` _returnvalue (struct :`TagName` "Player.Status.BounceLargeBullet")) :`false` "/Game/Blueprints/Abilities/GE_PerfectBounce.GE_PerfectBounce_C" :`true` "/Game/Blueprints/Abilities/GE_PerfectBounceScale.GE_PerfectBounceScale_C" :!type "GameplayEffect Class Reference"))
          (set `self.Cooldown` (`self.SuccessCooldown`))
          (`self.K2_CommitAbility`)
          (`|ExecutionSequence`
            (:`then_0`
              (`self.K2_ExecuteGameplayCueWithParams` (struct :`TagName` "GameplayCue.Bullet.PerfectBounce") (`AbilitySystemBlueprintLibrary.MakeGameplayCueParameters` 0.0 0.0 (struct) (struct) (struct) (struct) (struct) (`Actor.K2_GetActorLocation` _output) (0.0 0.0 0.0) null null _output)))
            (:`then_1`
              (`self.K2_EndAbility`))))))
    (:`OnFinish`
      (bind _bouncetask (`self.BounceTask`)
        (:`then`
          (`GameplayTask.EndTask` _bouncetask))
        (:`else`
          _))
      (set `self.Cooldown` (`self.FailCooldown`))
      (bind _asdonplayer_character (cast `DONPlayerCharacter` (`self.GetOwningActorFromActorInfo`))
        (:`then`
          _)
        (:`CastFailed`
          _))
      (`self.K2_CommitAbility`)
      (`self.K2_ExecuteGameplayCueWithParams` (struct :`TagName` "GameplayCue.Bullet.FailBounce") (`AbilitySystemBlueprintLibrary.MakeGameplayCueParameters` 0.0 0.0 (struct) (struct) (struct) (struct) (struct) (0.0 0.0 0.0) (0.0 0.0 0.0) null null (`KismetArrayLibrary.Array_Random` (`DONPlayerCharacter.Bullets` _asdonplayer_character))))
      (`self.K2_EndAbility`))))

(event `self.K2_OnEndAbility`
  (params (bWasCancelled :type Boolean))
  (bind _waittask (`self.WaitTask`)
    (:`then`
      (`GameplayTask.EndTask` _waittask)
      (bind _bouncetask (`self.BounceTask`)
        (:`then`
          (`GameplayTask.EndTask` _bouncetask))
        (:`else`)))
    (:`else`)))