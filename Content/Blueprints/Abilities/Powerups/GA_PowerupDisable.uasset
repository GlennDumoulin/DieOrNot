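; GA_PowerupDisable is a Gameplay Ability for a powerup that applies a disable effect to players.
; On activation it commits, then loops over the GameState PlayerArray and applies GE_PowerupDisableApply to each pawn's ability system, with no filter excluding the user.
; It then fires the GameplayCue.Powerup.Disable cue and ends the ability, which also ends immediately if the commit fails.
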(event `self.K2_ActivateAbility`
  (bind _returnvalue (`self.K2_CommitAbility`))
  (if _returnvalue
    (`self.ApplyEffectToAllPlayers`)
    (`self.K2_ExecuteGameplayCue` (struct :`TagName` "GameplayCue.Powerup.Disable")))
  (`self.K2_EndAbility`))

(fn `ApplyEffectToAllPlayers`
  (for _array_element (`GameStateBase.PlayerArray` (`GameplayStatics.GetGameState`))
    (`AbilitySystemComponent.BP_ApplyGameplayEffectToSelf` :`self` (`AbilitySystemBlueprintLibrary.GetAbilitySystemComponent` (`PlayerState.GetPawn` _array_element)) :`GameplayEffectClass` "/Game/Blueprints/Abilities/Powerups/GE_PowerupDisableApply.GE_PowerupDisableApply_C" :`Level` 1.0))
  (return))