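; GA_PowerupShootAgain is a Gameplay Ability for the Shoot Again powerup that clears the bullets tracked by the player character.
; Once the ability commits, it casts the avatar to BP_PlayerCharacter and loops over its Bullets array.
; It fires the ShootAgain gameplay cue at each bullet's location, destroys that bullet, and ends after the loop.
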(event `self.K2_ActivateAbility`
  (bind _returnvalue (`self.K2_CommitAbility`))
  (if _returnvalue
    (bind _asbp_player_character (cast `/Game/Blueprints/Gameplay/BP_PlayerCharacter` (`self.GetAvatarActorFromActorInfo`)))
    (for _array_element (`DONPlayerCharacter.Bullets` _asbp_player_character)
      (`self.K2_ExecuteGameplayCueWithParams` (struct :`TagName` "GameplayCue.Powerup.ShootAgain") (`AbilitySystemBlueprintLibrary.MakeGameplayCueParameters` 0.0 0.0 (struct) (struct) (struct) (struct) (struct) (`Actor.K2_GetActorLocation` _array_element)))
      (`DONBullet.DestroyBullet` _array_element))
    (`self.K2_EndAbility`)
    (else
      (`self.K2_EndAbility`))))