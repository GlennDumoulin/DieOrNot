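; GA_PowerupSafeZone is a gameplay ability powerup that clears nearby bullets around the player.
; After committing, it runs a zero-length multi-sphere trace over WorldDynamic objects at the avatar's location and destroys each BP_Bullet it hits.
; It then executes the SafeZone gameplay cue and ends, a step that also runs when the commit fails.
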(event `self.K2_ActivateAbility`
  (bind _returnvalue (`self.K2_CommitAbility`))
  (if _returnvalue
    (bind _asbp_player_character (cast `/Game/Blueprints/Gameplay/BP_PlayerCharacter` (`self.GetAvatarActorFromActorInfo`)))
    (bind _returnvalue_2 (`Actor.K2_GetActorLocation` _asbp_player_character))
    (bind _outhits (`KismetSystemLibrary.SphereTraceMultiForObjects` :`Start` _returnvalue_2 :`End` _returnvalue_2 :`Radius` 500.0 :`ObjectTypes` (`|MakeArray` "ObjectTypeQuery2" :!type "EObjectTypeQuery Enum") :`DrawTime` 0.2))
    (for _array_element _outhits
      (bind _asbp_bullet (cast `/Game/Blueprints/Gameplay/BP_Bullet` (`.HitActor` (`GameplayStatics.BreakHitResult` _array_element))))
      (`DONBullet.DestroyBullet` _asbp_bullet)))
  (`self.K2_ExecuteGameplayCue` (struct :`TagName` "GameplayCue.Powerup.SafeZone"))
  (`self.K2_EndAbility`))