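; Gameplay ability for the laser powerup that turns each of the player character's bullets into a forward laser beam.
; On activation it fires a laser gameplay cue per bullet and sphere-traces along its heading.
; Hit players get a kill attempt, hit bullets are destroyed, platforms take massive damage, then the source bullet is destroyed.
; A helper that ends the trace at the level border exists but is not called here.
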(event `self.K2_ActivateAbility`
  (bind _returnvalue (`self.K2_CommitAbility`))
  (if _returnvalue
    (bind _asbp_player_character (cast `/Game/Blueprints/Gameplay/BP_PlayerCharacter` (`self.GetAvatarActorFromActorInfo`))
      (:`then`
        (for _array_element (`DONPlayerCharacter.Bullets` _asbp_player_character)
          (bind (_returnvalue_location _returnvalue_rotation) (`KismetMathLibrary.BreakTransform` (`Actor.GetTransform` _array_element)))
          (bind _returnvalue_2 (+ _returnvalue_location (* (`KismetMathLibrary.Conv_RotatorToVector` _returnvalue_rotation) 5000.0)))
          (bind _returnvalue_3 (- _returnvalue_2 _returnvalue_location))
          (`self.K2_ExecuteGameplayCueWithParams` (struct :`TagName` "GameplayCue.Powerup.Laser") (`AbilitySystemBlueprintLibrary.MakeGameplayCueParameters` 0.0 (`KismetMathLibrary.VSize` _returnvalue_3) (struct) (struct) (struct) (struct) (struct) _returnvalue_location (`KismetMathLibrary.Normal` _returnvalue_3) null null _array_element))
          (bind _outhits (`KismetSystemLibrary.SphereTraceMultiForObjects` _returnvalue_location _returnvalue_2 50.0 (`|MakeArray` "ObjectTypeQuery2" "ObjectTypeQuery3" "ObjectTypeQuery1" :!type "EObjectTypeQuery Enum") false (`|MakeArray` _array_element :!type "Actor Object Reference") "None" false (struct :`R` 1.0 :`A` 1.0) (struct :`G` 1.0 :`A` 1.0) 0.2))
          (for _array_element_2 _outhits
            (bind (_bblockinghit _binitialoverlap _time _distance _location _impactpoint _normal _impactnormal _physmat _hitactor) (`GameplayStatics.BreakHitResult` _array_element_2))
            (bind _asbp_player_character_2 (cast `/Game/Blueprints/Gameplay/BP_PlayerCharacter` _hitactor)
              (:`then`
                (`DONPlayerCharacter.TryKillPlayer` _asbp_player_character_2 _array_element))
              (:`CastFailed`
                (bind _asbp_bullet (cast `/Game/Blueprints/Gameplay/BP_Bullet` _hitactor)
                  (:`then`
                    (`DONBullet.DestroyBullet` _asbp_bullet))
                  (:`CastFailed`
                    (bind _asbp_platform (cast `/Game/Blueprints/Level/BP_Platform` _hitactor))
                    (`/Game/Blueprints/Level/BP_Platform.TakeDamage` _asbp_platform 10000.0 _location))))))
          (`/Engine/EditorBlueprintResources/StandardMacros.IsValid` _array_element
            (:`Is Valid`
              (`DONBullet.DestroyBullet` _array_element)))))
      (:`CastFailed`
        _)))
  (`self.K2_EndAbility`))

(event `self.K2_OnEndAbility`
  (params (bWasCancelled :type Boolean)))

(fn `Get Trace Start and End`
  (params (BulletActor :type "DONBullet Object Reference"))
  (returns (TraceStart :type "Vector Structure") (TraceEnd :type "Vector Structure") (Success :type Boolean))
  (bind (_returnvalue_location _returnvalue_rotation) (`KismetMathLibrary.BreakTransform` (`Actor.GetTransform` BulletActor)))
  (bind _outhits (`KismetSystemLibrary.LineTraceMultiForObjects` _returnvalue_location (+ _returnvalue_location (* (`KismetMathLibrary.Conv_RotatorToVector` _returnvalue_rotation) 10000.0)) (`|MakeArray` "ObjectTypeQuery1" :!type "EObjectTypeQuery Enum")))
  (for _array_element _outhits
    (bind (_bblockinghit _binitialoverlap _time _distance _location _impactpoint _normal _impactnormal _physmat _hitactor _hitcomponent) (`GameplayStatics.BreakHitResult` _array_element))
    (bind _asstatic_mesh_component (cast `StaticMeshComponent` _hitcomponent))
    (if (== (`StaticMeshComponent.StaticMesh` _asstatic_mesh_component) "/Game/Assets/LevelAssets/Meshes/SM_LevelBorderBig.SM_LevelBorderBig")
      (return _returnvalue_location _location true)))
  (return (0.0 0.0 0.0) (0.0 0.0 0.0) false))