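; BP_OilSpill is a temporary oil spill effect actor with looping audio, a spill effect and a decal.
; On begin play it fades the audio in, runs the spill for a few seconds, then deactivates it and fades the audio out.
; The decal then fades and destroys the actor.
; A binding to the game mode's round-end event destroys it early when the round ends.
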(event `self.ReceiveBeginPlay`
  (add `/Game/Blueprints/Gameplay/BP_Gamemode.OnRoundEndEvent` (cast `/Game/Blueprints/Gameplay/BP_Gamemode` (`GameplayStatics.GetGameMode`) :!pure true) (delegate `End`))
  (`AudioComponent.FadeIn` (`self.Audio`) 0.5 1.0 0.0 "Linear")
  (`KismetSystemLibrary.Delay` 3.0)
  (`ActorComponent.Deactivate` (`self.Spill`))
  (`AudioComponent.FadeOut` (`self.Audio`) 0.5 0.0 "Linear")
  (`KismetSystemLibrary.Delay` 1.0)
  (`DecalComponent.SetFadeOut` (`self.Decal`) 0.0 1.0 true))

(event `End`
  (`self.K2_DestroyActor`))

(event `self.Audio.OnAudioFinished`
  (`AudioComponent.Play` (`self.Audio`) 0.0))

(fn `UserConstructionScript`)