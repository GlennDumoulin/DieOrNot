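; Destructible level platform that takes damage from fast-moving actors hitting it, active only when challenges are enabled.
; Impact speed sets damage, scaled down for DONPlayerCharacter hits, and max health rises with more than two players.
; The Light decal shrinks with health, flashing red and shaking on hits.
; At depleted health, Base swaps to the physics-simulated Breakable, shattered by a temporary FS_MasterField with camera shake and crumble sound.
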(event `self.ReceiveBeginPlay`
  (bind _maxhealth (`self.MaxHealth`))
  (if (`DONGameInstance.GetEnableChallenges` (cast `DONGameInstance` (`GameplayStatics.GetGameInstance`) :!pure true))
    (add `PrimitiveComponent.OnComponentHit` (`self.Base`) (delegate `OnComponentHit_Event`))
    (set `self.StartScale` (`SceneComponent.K2_GetComponentScale` (`self.Light`)))
    (bind _output_get (set `self.MaxHealth` (`KismetMathLibrary.SelectFloat` (* _maxhealth 1.5) _maxhealth (> (`GameplayStatics.GetNumPlayerStates`) 2))))
    (set `self.Health` _output_get)
    (bind _returnvalue (`DecalComponent.CreateDynamicMaterialInstance` (`self.Light`)))
    (set `self.DecalMaterial` _returnvalue)
    (set `self.EnableDamage` (`DONGameInstance.GetEnableChallenges` (cast `DONGameInstance` (`GameplayStatics.GetGameInstance`) :!pure true)))))

(event `OnComponentHit_Event`
  (params (HitComponent :type "PrimitiveComponent Object Reference") (OtherActor :type "Actor Object Reference") (OtherComp :type "PrimitiveComponent Object Reference") (NormalImpulse :type "Vector Structure") (Hit :type "HitResult Structure (by ref)"))
  (bind _returnvalue (`KismetMathLibrary.VSize` (`self.GetVelocity` OtherActor)))
  (if (and (> _returnvalue 300.0) (`self.CanTakeDamage`))
    (set `self.CanTakeDamage` false)
    (`self.TakeDamage` (`KismetMathLibrary.SelectFloat` (* _returnvalue 0.6) _returnvalue (`.bSuccess` (cast `DONPlayerCharacter` OtherActor :!pure true))) (`.Location` (`GameplayStatics.BreakHitResult` Hit)))
    (`KismetSystemLibrary.Delay` 0.2)
    (set `self.CanTakeDamage` true)))

(event `TakeDamage`
  (params (B :type "Float (double-precision)") (Location :type "Vector Structure"))
  (bind _decalmaterial (`self.DecalMaterial`))
  (bind _light (`self.Light`))
  (bind (_startscale_x _startscale_y _startscale_z) (`KismetMathLibrary.BreakVector` (`self.StartScale`)))
  (if (`self.EnableDamage`)
    (bind _output_get (set `self.Health` (- (`self.Health`) B)))
    (`SceneComponent.SetWorldScale3D` _light (`KismetMathLibrary.MakeVector` _startscale_x _startscale_y (`KismetMathLibrary.FClamp` (* _startscale_z (/ (`self.Health`) (`self.MaxHealth`))) 0.0 _startscale_z)))
    (if (< _output_get 0.0)
      (`self.Break` Location)
      (`SceneComponent.SetHiddenInGame` _light true false)
      (else
        (`|ExecutionSequence`
          (:`then_0`
            (`MaterialInstanceDynamic.SetVectorParameterValue` _decalmaterial "Color" (struct :`R` 1.0 :`A` 1.0))
            (`KismetSystemLibrary.RetriggerableDelay` 0.1)
            (`MaterialInstanceDynamic.SetVectorParameterValue` _decalmaterial "Color" (struct :`R` 1.0 :`G` 1.0 :`B` 1.0 :`A` 1.0)))
          (:`then_1`
            (bind (_direction _newtrack_0) (`Timeline|Shake` :!via `PlayFromStart`)
              (:`Update`
                (`SceneComponent.K2_SetRelativeLocation` (`self.Light`) (`KismetMathLibrary.MakeVector` 0.0 0.0 (* _newtrack_0 5.0)) false false)))))))))

(event `ResetPlatform`)

(event `Break`
  (params (Location :type "Vector Structure"))
  (bind _base (`self.Base`))
  (bind _breakable (`self.Breakable`))
  (`|ExecutionSequence`
    (:`then_0`
      (`PrimitiveComponent.SetCollisionEnabled` (`self.Breakable`) "QueryAndPhysics")
      (`PrimitiveComponent.SetCollisionEnabled` _base "NoCollision")
      (`SceneComponent.SetHiddenInGame` _base true false)
      (`SceneComponent.SetHiddenInGame` _breakable false false)
      (`PrimitiveComponent.SetSimulatePhysics` _breakable true)
      (bind _returnvalue (`|SpawnActorFromClass` "/Engine/EditorResources/FieldNodes/FS_MasterField.FS_MasterField_C" (`KismetMathLibrary.MakeTransform` Location (struct) (4.0 4.0 4.0)) "AlwaysSpawn" "OverrideRootScale" null null))
      (set `/Engine/EditorResources/FieldNodes/FS_MasterField.ActivationType` "NewEnumerator4" _returnvalue)
      (set `/Engine/EditorResources/FieldNodes/FS_MasterField.Radial Magnitude` 500.0 _returnvalue)
      (`/Engine/EditorResources/FieldNodes/FS_MasterField.CE_Trigger` _returnvalue)
      (`KismetSystemLibrary.Delay` 1.0)
      (`self.K2_DestroyActor` _returnvalue))
    (:`then_1`
      (`PlayerController.ClientStartCameraShake` :`self` (`GameplayStatics.GetPlayerController` 0) :`Shake` "/Game/Blueprints/CameraShakes/BP_PlatformShake.BP_PlatformShake_C")
      (`GameplayStatics.PlaySoundAtLocation` "/Game/SFX/Game/SW_PlatformCrumble.SW_PlatformCrumble" (`self.K2_GetActorLocation`) (struct) 1.0 1.0 0.0 null null null null))))

(fn `UserConstructionScript`)