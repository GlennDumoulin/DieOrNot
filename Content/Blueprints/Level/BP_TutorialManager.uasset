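; Tutorial manager that teaches local players dash, bullet redirect, power bounce and parry through pop-up prompts during play.
; Each lesson picks players via jump or bullet-spawn events, or colliders attached at runtime to bullets and players.
; Triggers freeze global time dilation and show WBP_TutorialFade until the player responds, using temporary Immortal tags and an input mapping context where needed.
; Redirect leads into power bounce, while parry also points out the charge pickup.
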(event `self.ReceiveDestroyed`)

(event `self.ReceiveBeginPlay`
  (`self.MakeRedirect`)
  (`self.MakeParry`)
  (`self.MakeDash`)
  (bind _returnvalue (`|CreateWidget` "/Game/Blueprints/UI/Tutorial/WBP_TutorialFade.WBP_TutorialFade_C" null self))
  (bind _output_get (set `self.HUD` _returnvalue))
  (`UserWidget.AddToViewport` _output_get 0)
  (`DONGameInstance.SetEnableTutorials` (cast `DONGameInstance` (`GameplayStatics.GetGameInstance`) :!pure true) false))

(event `MakeDash`
  ;[1 1 1] Dash
  (if (not (`self.DashComplete`))
    (bind _asbp_player_character (`self.GetRandomPlayer`))
    (bind _output_get (set `self.DashPlayer` _asbp_player_character))
    (add `/Game/Blueprints/Gameplay/BP_PlayerCharacter.OnJump` _output_get (delegate `DashTutorial`))))

(event `DestroyComponent` :!signature `self.OnDestroyed`
  (params (DestroyedActor :type "Actor Object Reference"))
  ;[1 1 1] Redirect
  (bind _bulletcollider (`self.BulletCollider`)
    (:`then`
      (`ActorComponent.K2_DestroyComponent` _bulletcollider)
      (bind _redirectplayer (`self.RedirectPlayer`)
        (:`then`
          (remove `/Game/Blueprints/Gameplay/BP_PlayerCharacter.OnTutorialAccept` _redirectplayer (delegate `CloseRedirect`)))
        (:`else`)))
    (:`else`)))

(event `MakeRedirect`
  ;[1 1 1] Redirect
  (if (not (`self.RedirectComplete`))
    (bind _asbp_player_character (`self.GetRandomPlayer`))
    (bind _output_get (set `self.RedirectPlayer` _asbp_player_character))
    (add `DONPlayerCharacter.OnBulletSpawned` _output_get (delegate `MakeBulletCollidr`))))

(event `DashTutorial`
  (bind _returnvalue (`BlueprintGameplayTagLibrary.MakeGameplayTagContainerFromTag` (struct :`TagName` "Player.Status.Immortal")))
  (bind _dashplayer (`self.DashPlayer`))
  (bind _hud (`self.HUD`))
  ;[1 1 1] Dash
  (if (and (`self.CanContinue`) (not (`self.TutorialInProgress`)))
    (`/Engine/EditorBlueprintResources/StandardMacros.FlipFlop`
      (:`A`
        (`/Engine/EditorBlueprintResources/StandardMacros.DoOnce` false :!label _label
          (:`Completed`
            (set `self.CanContinue` false)
            (`AbilitySystemBlueprintLibrary.AddLooseGameplayTags` _dashplayer _returnvalue)
            (`KismetSystemLibrary.Delay` 0.3)
            (if (`DONPlayerCharacter.bAlive` _dashplayer)
              (`GameplayStatics.SetGlobalTimeDilation` 0.0)
              (`/Game/Blueprints/UI/Tutorial/WBP_TutorialFade.Show` _hud true _dashplayer "/Game/Textures/UI/XBoxControllerIcons/XboxSeriesX_A.XboxSeriesX_A" "Press jump while in air to dash" (`self.K2_GetActorLocation` _dashplayer))
              (set `self.DashComplete` true)
              (else
                (goto _label :!via `Reset`))))))
      (:`B`
        (`GameplayStatics.SetGlobalTimeDilation` 1.0)
        (remove `/Game/Blueprints/Gameplay/BP_PlayerCharacter.OnJump` _dashplayer (delegate `DashTutorial`))
        (`AbilitySystemBlueprintLibrary.RemoveLooseGameplayTags` _dashplayer _returnvalue)
        (`/Game/Blueprints/UI/Tutorial/WBP_TutorialFade.Show` _hud false null null "" (0.0 0.0 0.0))
        (set `self.CanContinue` true)))))

(event `MakeBulletCollidr`
  (params (Bullet :type "DONBullet Object Reference"))
  ;[1 1 1] Redirect
  (remove `DONPlayerCharacter.OnBulletSpawned` (`self.RedirectPlayer`) (delegate `MakeBulletCollidr`))
  (bind _returnvalue (`|AddComponentByClass` "/Script/Engine.CapsuleComponent" true (`KismetMathLibrary.MakeTransform` (80.0 0.0 0.0) (struct :`Pitch` 90.0))))
  (bind _output_get (set `self.BulletCollider` _returnvalue))
  (`SceneComponent.K2_AttachToComponent` _returnvalue (`Actor.RootComponent` Bullet) "None" "KeepRelative" "KeepRelative" "KeepRelative" true)
  (add `self.OnDestroyed` Bullet (delegate `DestroyComponent`))
  (`PrimitiveComponent.SetCollisionResponseToAllChannels` _output_get "ECR_Ignore")
  (`PrimitiveComponent.SetCollisionResponseToChannel` _output_get "ECC_WorldStatic" "ECR_Overlap")
  (`CapsuleComponent.SetCapsuleSize` _output_get 20.0 80.0 true)
  (`KismetSystemLibrary.Delay` 6.0)
  (add `PrimitiveComponent.OnComponentBeginOverlap` _output_get (delegate `Redirect`)))

(event `Redirect`
  (params (OverlappedComponent :type "PrimitiveComponent Object Reference") (OtherActor :type "Actor Object Reference") (OtherComp :type "PrimitiveComponent Object Reference") (OtherBodyIndex :type Integer) (bFromSweep :type Boolean) (SweepResult :type "HitResult Structure (by ref)"))
  (bind _bulletcollider (`self.BulletCollider`))
  (bind _redirectplayer (`self.RedirectPlayer`))
  ;[1 1 1] Redirect
  (set `self.TutorialInProgress` true)
  (`GameplayStatics.SetGlobalTimeDilation` 0.0)
  (`/Game/Blueprints/UI/Tutorial/WBP_TutorialFade.Show` (`self.HUD`) true _redirectplayer "/Game/Textures/UI/XBoxControllerIcons/XboxSeriesX_A.XboxSeriesX_A" "Redirect bullet during bounces with right stick" (`SceneComponent.K2_GetComponentLocation` _bulletcollider))
  (`ActorComponent.K2_DestroyComponent` _bulletcollider)
  (add `/Game/Blueprints/Gameplay/BP_PlayerCharacter.OnTutorialAccept` _redirectplayer (delegate `CloseRedirect`))
  (set `self.CanContinue` false)
  (set `self.RedirectComplete` true)
  (message `EnhancedInputSubsystemInterface.AddMappingContext` (pcsubsystem `EnhancedInputLocalPlayerSubsystem` (cast `PlayerController` (`Pawn.GetController` (`self.RedirectPlayer`)) :!pure true)) "/Game/Blueprints/Input/IM_TutorialMapping.IM_TutorialMapping" 10 (make `ModifyContextOptions` true)))

(event `CloseRedirect`
  ;[1 1 1] Redirect
  (if (`self.CanContinue`)
    (`/Game/Blueprints/UI/Tutorial/WBP_TutorialFade.Show` (`self.HUD`) false null "/Game/Textures/UI/XBoxControllerIcons/XboxSeriesX_A.XboxSeriesX_A" "" (0.0 0.0 0.0))
    (remove `/Game/Blueprints/Gameplay/BP_PlayerCharacter.OnTutorialAccept` (`self.RedirectPlayer`) (delegate `CloseRedirect`))
    (`GameplayStatics.SetGlobalTimeDilation` 1.0)
    (message `EnhancedInputSubsystemInterface.RemoveMappingContext` (pcsubsystem `EnhancedInputLocalPlayerSubsystem` (cast `PlayerController` (`Pawn.GetController` (`self.RedirectPlayer`)) :!pure true)) "/Game/Blueprints/Input/IM_TutorialMapping.IM_TutorialMapping" (make `ModifyContextOptions` true))
    (`self.PowerBounceTutorial`)
    (set `self.TutorialInProgress` false)))

(event `PowerBounceTutorial`
  ;[1 1 1] Bounce
  (bind _outactors (`GameplayStatics.GetAllActorsOfClass` "/Game/Blueprints/Gameplay/BP_Bullet.BP_Bullet_C"))
  (if (`KismetArrayLibrary.Array_IsEmpty` _outactors)
    (if (not (`self.BounceComplete`))
      (bind _asbp_player_character (`self.GetRandomPlayer`))
      (bind _output_get (set `self.RedirectPlayer` _asbp_player_character))
      (add `DONPlayerCharacter.OnBulletSpawned` _output_get (delegate `BounceSpawn`)))
    (else
      (`self.BounceSpawn` (`KismetArrayLibrary.Array_Random` _outactors)))))

(event `BounceSpawn`
  (params (Bullet :type "DONBullet Object Reference"))
  ;[1 1 1] Bounce
  (set `self.RedirectPlayer` (cast `/Game/Blueprints/Gameplay/BP_PlayerCharacter` (`DONBullet.PlayerOwner` Bullet) :!pure true))
  (remove `DONPlayerCharacter.OnBulletSpawned` (`self.RedirectPlayer`) (delegate `BounceSpawn`))
  (bind _returnvalue (`|AddComponentByClass` "/Script/Engine.CapsuleComponent" false (`KismetMathLibrary.MakeTransform` (80.0 0.0 0.0) (struct :`Pitch` 90.0))))
  (bind _output_get (set `self.BounceCollider` _returnvalue))
  (`SceneComponent.K2_AttachToComponent` _returnvalue (`Actor.RootComponent` Bullet) "None" "KeepRelative" "KeepRelative" "KeepRelative" true)
  (`PrimitiveComponent.SetCollisionResponseToAllChannels` _output_get "ECR_Ignore")
  (`PrimitiveComponent.SetCollisionResponseToChannel` _output_get "ECC_WorldStatic" "ECR_Overlap")
  (`CapsuleComponent.SetCapsuleSize` _output_get 20.0 80.0 true)
  (`KismetSystemLibrary.Delay` 6.0)
  (add `PrimitiveComponent.OnComponentBeginOverlap` _output_get (delegate `BounceOverlap`)))

(event `BounceOverlap`
  (params (OverlappedComponent :type "PrimitiveComponent Object Reference") (OtherActor :type "Actor Object Reference") (OtherComp :type "PrimitiveComponent Object Reference") (OtherBodyIndex :type Integer) (bFromSweep :type Boolean) (SweepResult :type "HitResult Structure (by ref)"))
  (bind _bouncecollider (`self.BounceCollider`))
  (bind _redirectplayer (`self.RedirectPlayer`))
  ;[1 1 1] Bounce
  (set `self.TutorialInProgress` true)
  (`GameplayStatics.SetGlobalTimeDilation` 0.0)
  (`/Game/Blueprints/UI/Tutorial/WBP_TutorialFade.Show` (`self.HUD`) true _redirectplayer "/Game/Textures/UI/XBoxControllerIcons/XboxSeriesX_RB.XboxSeriesX_RB" "Press right shoulder to bounce perfectly" (`SceneComponent.K2_GetComponentLocation` _bouncecollider))
  (`ActorComponent.K2_DestroyComponent` _bouncecollider)
  (add `DONPlayerCharacter.OnBounceActivated` _redirectplayer (delegate `CloseBounce`))
  (set `self.CanContinue` false)
  (set `self.BounceComplete` true))

(event `CloseBounce`
  ;[1 1 1] Bounce
  (if (`self.CanContinue`)
    (`/Game/Blueprints/UI/Tutorial/WBP_TutorialFade.Show` (`self.HUD`) false null "/Game/Textures/UI/XBoxControllerIcons/XboxSeriesX_A.XboxSeriesX_A" "" (0.0 0.0 0.0))
    (remove `DONPlayerCharacter.OnBounceActivated` (`self.RedirectPlayer`) (delegate `CloseBounce`))
    (`GameplayStatics.SetGlobalTimeDilation` 1.0)
    (set `self.TutorialInProgress` false)))

(event `MakeParry`
  ;[1 1 1] Parry
  (`KismetSystemLibrary.Delay` 6.0)
  (if (not (`self.ParryComplete`))
    (bind _asbp_player_character (`self.GetRandomPlayer`))
    (bind _output_get (set `self.ParryPlayer` _asbp_player_character))
    (bind _returnvalue (`|AddComponentByClass` "/Script/Engine.SphereComponent" true))
    (bind _output_get_2 (set `self.ParryCollider` _returnvalue))
    (`SceneComponent.K2_AttachToComponent` _output_get_2 (`Actor.RootComponent` _output_get) "None" "KeepRelative" "KeepRelative" "KeepRelative" true)
    (`SphereComponent.SetSphereRadius` _output_get_2 80.0 false)
    (`PrimitiveComponent.SetCollisionResponseToAllChannels` _output_get_2 "ECR_Ignore")
    (`PrimitiveComponent.SetCollisionResponseToChannel` _output_get_2 "ECC_WorldDynamic" "ECR_Overlap")
    (add `PrimitiveComponent.OnComponentBeginOverlap` _output_get_2 (delegate `ParryOverlap`))))

(event `ParryOverlap`
  (params (OverlappedComponent :type "PrimitiveComponent Object Reference") (OtherActor :type "Actor Object Reference") (OtherComp :type "PrimitiveComponent Object Reference") (OtherBodyIndex :type Integer) (bFromSweep :type Boolean) (SweepResult :type "HitResult Structure (by ref)"))
  (bind _parrycollider (`self.ParryCollider`))
  (bind _parryplayer (`self.ParryPlayer`))
  (bind _parryplayer_2 (`self.ParryPlayer`))
  ;[1 1 1] Parry
  (cast `/Game/Blueprints/Gameplay/BP_Bullet` OtherActor)
  (if (and (`GameplayTagAssetInterface.HasMatchingGameplayTag` (`DONPlayerCharacter.AbilitySystemComponent` _parryplayer) (struct :`TagName` "Player.Status.Parry")) (> (`KismetMathLibrary.Dot_VectorVector` (`self.GetActorForwardVector` OtherActor) (`KismetMathLibrary.Normal` (- (`self.K2_GetActorLocation` _parryplayer) (`self.K2_GetActorLocation` OtherActor)))) 0.0) (`DONPlayerCharacter.bAlive` _parryplayer))
    (`AbilitySystemBlueprintLibrary.AddLooseGameplayTags` _parryplayer (`BlueprintGameplayTagLibrary.MakeGameplayTagContainerFromTag` (struct :`TagName` "Player.Status.Immortal")))
    (set `self.TutorialInProgress` true)
    (`GameplayStatics.SetGlobalTimeDilation` 0.0)
    (`/Game/Blueprints/UI/Tutorial/WBP_TutorialFade.Show` (`self.HUD`) true _parryplayer_2 "/Game/Textures/UI/XBoxControllerIcons/XboxSeriesX_LT.XboxSeriesX_LT" "Press left trigger to parry incoming bullets" (`SceneComponent.K2_GetComponentLocation` _parrycollider))
    (`ActorComponent.K2_DestroyComponent` _parrycollider)
    (add `DONPlayerCharacter.OnParryActivated` _parryplayer_2 (delegate `ParryTutorialEnd`))
    (set `self.CanContinue` false)
    (set `self.ParryComplete` true)))

(event `ParryTutorialEnd`
  (bind _parryplayer (`self.ParryPlayer`))
  ;[1 1 1] Parry
  (if (`self.CanContinue`)
    (`AbilitySystemBlueprintLibrary.RemoveLooseGameplayTags` (`self.ParryPlayer`) (`BlueprintGameplayTagLibrary.MakeGameplayTagContainerFromTag` (struct :`TagName` "Player.Status.Immortal")) true)
    (bind _returnvalue (`GameplayStatics.GetActorOfClass` "/Game/Blueprints/Gameplay/Pickups/BP_ParryPickup.BP_ParryPickup_C"))
    (`/Game/Blueprints/UI/Tutorial/WBP_TutorialFade.Show` (`self.HUD`) true _parryplayer "/Game/Textures/UI/XBoxControllerIcons/XboxSeriesX_A.XboxSeriesX_A" "Collect charges here" (`self.K2_GetActorLocation` _returnvalue))
    (remove `DONPlayerCharacter.OnParryActivated` _parryplayer (delegate `ParryTutorialEnd`))
    (add `/Game/Blueprints/Gameplay/BP_PlayerCharacter.OnTutorialAccept` _parryplayer (delegate `CloseParry`))
    (set `self.CanContinue` false)
    (message `EnhancedInputSubsystemInterface.AddMappingContext` (pcsubsystem `EnhancedInputLocalPlayerSubsystem` (cast `PlayerController` (`Pawn.GetController` (`self.ParryPlayer`)) :!pure true)) "/Game/Blueprints/Input/IM_TutorialMapping.IM_TutorialMapping" 10 (make `ModifyContextOptions` true))))

(event `CloseParry`
  ;[1 1 1] Parry
  (if (`self.CanContinue`)
    (`/Game/Blueprints/UI/Tutorial/WBP_TutorialFade.Show` (`self.HUD`) false null "/Game/Textures/UI/XBoxControllerIcons/XboxSeriesX_A.XboxSeriesX_A" "Collect charges here" (0.0 0.0 0.0))
    (remove `/Game/Blueprints/Gameplay/BP_PlayerCharacter.OnTutorialAccept` (`self.ParryPlayer`) (delegate `CloseParry`))
    (message `EnhancedInputSubsystemInterface.RemoveMappingContext` (pcsubsystem `EnhancedInputLocalPlayerSubsystem` (cast `PlayerController` (`Pawn.GetController` (`self.ParryPlayer`)) :!pure true)) "/Game/Blueprints/Input/IM_TutorialMapping.IM_TutorialMapping" (make `ModifyContextOptions` true))
    (`GameplayStatics.SetGlobalTimeDilation` 1.0)
    (set `self.TutorialInProgress` false)))

(fn `GetRandomPlayer`
  (returns (`AsBP Player Character` :type "/Game/Blueprints/Gameplay/BP_PlayerCharacter Object Reference"))
  (return (cast `/Game/Blueprints/Gameplay/BP_PlayerCharacter` (`GameplayStatics.GetPlayerCharacter` (`KismetMathLibrary.RandomIntegerInRange` 0 (- (`GameplayStatics.GetNumPlayerControllers`) 1))) :!pure true)))

(fn `UserConstructionScript`)