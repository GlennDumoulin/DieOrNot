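; BP_LevelCamera is the level's view camera, turning to follow the action and zooming in on the round winner.
; A looping timer gathers living player characters and bullets.
; While ShouldMove is set, Tick eases the look-at point toward a damped, downward-offset average of their locations, rotating the camera rather than moving it.
; RoundEnd retargets the winner and narrows FOV through the Zoom timeline, which reverses after a short hold.
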(event `self.ReceiveBeginPlay`
  (`KismetSystemLibrary.DelayUntilNextTick`)
  (`PlayerController.SetViewTargetWithBlend` (`GameplayStatics.GetPlayerController` 0) self 0.0 "VTBlend_Linear" 0.0 false)
  (`KismetSystemLibrary.K2_SetTimerDelegate` (delegate `Set Target`) 1.0 true)
  (`KismetSystemLibrary.Delay` 0.1)
  (`self.Set Target`)
  (set `self.BaseFOV` (`CameraComponent.FieldOfView` (`self.Camera`))))

(event `Set Target`
  (bind _actors (`self.Actors`))
  (`KismetArrayLibrary.Array_Clear` (`self.Actors`))
  (bind _outactors (`GameplayStatics.GetAllActorsOfClass` "/Game/Blueprints/Gameplay/BP_PlayerCharacter.BP_PlayerCharacter_C"))
  (for _array_element _outactors
    (if (`DONPlayerCharacter.bAlive` _array_element)
      (`KismetArrayLibrary.Array_Add` _actors _array_element)))
  (bind _outactors_2 (`GameplayStatics.GetAllActorsOfClass` "/Game/Blueprints/Gameplay/BP_Bullet.BP_Bullet_C"))
  (`KismetArrayLibrary.Array_Append` _actors _outactors_2))

(event `self.ReceiveTick`
  (params (DeltaSeconds :type "Float (single-precision)"))
  (bind _camera (`self.Camera`))
  (if (`self.ShouldMove`)
    (bind _output_get (set `self.Current` (`KismetMathLibrary.VInterpTo` (`self.Current`) (`self.TargetLoc`) DeltaSeconds 3.0)))
    (`SceneComponent.K2_SetWorldRotation` _camera (`KismetMathLibrary.FindLookAtRotation` (`SceneComponent.K2_GetComponentLocation` _camera) _output_get) false false)
    (if (not (`self.Zooming`))
      (bind _returnvalue (`GameplayStatics.GetActorArrayAverageLocation` (`self.Actors`)))
      (set `self.TargetLoc` (+ (* _returnvalue 0.1) (0.0 0.0 -140.0))))))

(event `RoundEnd`
  (params (Game :type "/Game/Blueprints/Gameplay/BP_Gamemode Object Reference"))
  (bind _winner (`DONGameModeBase.Winner` Game))
  (`/Engine/EditorBlueprintResources/StandardMacros.IsValid` _winner
    (:`Is Valid`
      (set `self.Zooming` true)
      (set `self.TargetLoc` (`self.K2_GetActorLocation` _winner))
      (bind (_direction _zoom) (`Timeline|Zoom` :!via `PlayFromStart` :!label _label)
        (:`Update`
          (`CameraComponent.SetFieldOfView` (`self.Camera`) (- (`self.BaseFOV`) (* _zoom 15.0))))
        (:`Finished`
          (if (`|EnumEquality` _direction "Forward")
            (`KismetSystemLibrary.Delay` 1.0)
            (set `self.Zooming` false)
            (goto _label :!via `ReverseFromEnd`)))))))

(event `RoundStart`
  (set `self.Zooming` false))

(fn `UserConstructionScript`)