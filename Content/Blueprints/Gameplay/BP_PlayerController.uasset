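; Player controller that opens and closes the pause menu, freezing and resuming the game.
; A GlobalPause key press and the IA_PauseGame input action share one toggle, which creates and focuses WBP_PauseMenu only if the game is not already paused.
; CloseMenu unpauses and removes the widget.
; Both paths tell BP_Gamemode to switch navigation mode on or off.
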(event `CloseMenu`
  (`GameplayStatics.SetGamePaused` false)
  (`Widget.RemoveFromParent` (`self.PauseMenu`))
  (set `self.MenuOpen` false)
  (set `self.PauseMenu` null)
  (`DONGameModeBase.SwitchNavigationMode` (cast `/Game/Blueprints/Gameplay/BP_Gamemode` (`GameplayStatics.GetGameMode`) :!pure true) false))

(event `Key|Global_Pause`
  (params (Key :type "Key Structure"))
  (:`Pressed`
    (if (`self.MenuOpen`) :!label _label
      (`/Engine/EditorBlueprintResources/StandardMacros.IsValid` (`self.PauseMenu`)
        (:`Is Valid`
          (`self.CloseMenu`)))
      (elif (not (`GameplayStatics.IsGamePaused`))
        (`GameplayStatics.SetGamePaused` true)
        (bind _returnvalue (`|CreateWidget` "/Game/Blueprints/UI/Game/WBP_PauseMenu.WBP_PauseMenu_C" self))
        (`UserWidget.AddToViewport` _returnvalue 0)
        (bind _output_get (set `self.PauseMenu` _returnvalue))
        (set `self.MenuOpen` true)
        (`/Game/Blueprints/UI/Common/WBP_FocusableRoot.SetPlayerFocus` _output_get self null)
        (`DONGameModeBase.SwitchNavigationMode` (cast `/Game/Blueprints/Gameplay/BP_Gamemode` (`GameplayStatics.GetGameMode`) :!pure true) true)))))

(event `EnhancedInput|/Game/Blueprints/Input/Actions/IA_PauseGame`
  (params (ActionValue :type Boolean) (ElapsedSeconds :type "Float (double-precision)") (TriggeredSeconds :type "Float (double-precision)") (InputAction :type "InputAction Object Reference" :default "/Game/Blueprints/Input/Actions/IA_PauseGame.IA_PauseGame"))
  (:`Triggered`
    (goto _label)))

(fn `UserConstructionScript`)