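; Player character Blueprint that turns Enhanced Input into movement, planar dash and aim directions, jumping, parry, bounce, powerup and tutorial actions.
; Input events mostly forward to functions defined outside this graph, with GAS attributes supplying jump and walk speed and GameplayCues firing jump and parry feedback.
; Movement-mode changes toggle walking effects and start coyote time.
; Head bones get half-blended physics; landing, victory and death trigger sound, montage or camera shake.
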(event `self.ReceiveBeginPlay`
  (bind _mesh (`self.Mesh`))
  (`|ExecutionSequence`
    (:`then_0`
      (`SkeletalMeshComponent.SetAllBodiesBelowSimulatePhysics` _mesh "Head_jnt" true true)
      (`SkeletalMeshComponent.SetAllBodiesBelowPhysicsBlendWeight` _mesh "Head_jnt" 0.5 true true))
    (:`then_1`
      (set `self.ParryComponent` (`self.ParryCollider`))
      (`self.DisableParry`))
    (:`then_2`
      (`AbilityAsync_WaitGameplayTagRemoved.WaitGameplayTagRemoveFromActor` null (struct :`TagName` "Player.Status.PowerupsBlocked")
        (:`Removed`
          (`self.RefreshHandle`)
          (`KismetSystemLibrary.PrintString` "Hello"))))))

(event `EnhancedInput|/Game/Blueprints/Input/Actions/IA_Move`
  (params (ActionValue :type "Vector2D Structure") (ElapsedSeconds :type "Float (double-precision)") (TriggeredSeconds :type "Float (double-precision)") (InputAction :type "InputAction Object Reference" :default "/Game/Blueprints/Input/Actions/IA_Move.IA_Move"))
  (bind (_x _y) (`KismetMathLibrary.BreakVector2D` ActionValue))
  ;[1 1 1] Player Movement
  (:`Triggered`
    (if (`self.bIsDashing`)
      (`self.MovePlayerCharacter` _x :!label _label)
      (else
        (`|ExecutionSequence`
          (:`then_0`
            (goto _label))
          (:`then_1`
            (set `self.DashDirection` (`KismetMathLibrary.MakeVector` 0.0 _x _y) :!label _label_2))))))
  (:`Completed`
    (goto _label_2)))

(event `EnhancedInput|/Game/Blueprints/Input/Actions/IA_AimBullet`
  (params (ActionValue :type "Vector2D Structure") (ElapsedSeconds :type "Float (double-precision)") (TriggeredSeconds :type "Float (double-precision)") (InputAction :type "InputAction Object Reference" :default "/Game/Blueprints/Input/Actions/IA_AimBullet.IA_AimBullet"))
  (bind (_x _y) (`KismetMathLibrary.BreakVector2D` ActionValue))
  ;[1 1 1] Handle Aiming
  (:`Triggered`
    (set `self.AimDirection` (`KismetMathLibrary.MakeVector` 0.0 _x _y)))
  (:`Completed`
    (set `self.AimDirection` (0.0 0.0 0.0))))

(event `EnhancedInput|/Game/Blueprints/Input/Actions/IA_Jump`
  (params (ActionValue :type Boolean) (ElapsedSeconds :type "Float (double-precision)") (TriggeredSeconds :type "Float (double-precision)") (InputAction :type "InputAction Object Reference" :default "/Game/Blueprints/Input/Actions/IA_Jump.IA_Jump"))
  (bind (_bsuccessfullyfoundattribute _returnvalue) (`AbilitySystemBlueprintLibrary.GetFloatAttribute` self (struct :`AttributeName` "JumpPower" :`Attribute` "/Script/DON.PlayerAttributeSet:JumpPower" :`AttributeOwner` "/Script/CoreUObject.Class'\"/Script/DON.PlayerAttributeSet\"'")))
  ;[1 1 1] Player Jumping/Dashing
  (:`Triggered`
    (if (`self.bAlive`)
      (`self.OnJump`)
      (bind _returnvalue_2 (`self.HandleJumping` (`KismetMathLibrary.SelectFloat` _returnvalue (`self.JumpVel`) _bsuccessfullyfoundattribute)))
      (if _returnvalue_2
        (`GameplayCueFunctionLibrary.ExecuteGameplayCueOnActor` self (struct :`TagName` "GameplayCue.Player.Jump") (`AbilitySystemBlueprintLibrary.MakeGameplayCueParameters` 0.0))))))

(event `self.OnLaunched`
  (params (LaunchVelocity :type "Vector Structure") (bXYOverride :type Boolean) (bZOverride :type Boolean))
  ;[1 1 1] Handle State Changes
  (`self.SetHasJumped` true))

(event `self.OnLanded`
  (params (Hit :type "HitResult Structure (by ref)"))
  ;[1 1 1] Handle State Changes
  (`self.SetHasJumped` false)
  (`GameplayStatics.PlaySoundAtLocation` "/Game/SFX/Game/SC_Landing_Cue.SC_Landing_Cue" (`self.K2_GetActorLocation`) (struct) 1.0 1.0 0.0 null null null null)
  (set `CharacterMovementComponent.MaxWalkSpeed` (`.ReturnValue` (`AbilitySystemBlueprintLibrary.GetFloatAttribute` self (struct :`AttributeName` "Speed" :`Attribute` "/Script/DON.PlayerAttributeSet:Speed" :`AttributeOwner` "/Script/CoreUObject.Class'\"/Script/DON.PlayerAttributeSet\"'"))) (`self.CharacterMovement`)))

(event `self.K2_OnMovementModeChanged`
  (params (PrevMovementMode :type "EMovementMode Enum" :default "MOVE_None") (NewMovementMode :type "EMovementMode Enum" :default "MOVE_None") (PrevCustomMode :type Byte) (NewCustomMode :type Byte))
  (bind _walkingeffect (`self.WalkingEffect`))
  ;[1 1 1] Handle Coyote Time
  (switch `EMovementMode` NewMovementMode
    (:`MOVE_Walking`
      (`ActorComponent.Activate` _walkingeffect false))
    (:`MOVE_Falling`
      (`ActorComponent.Deactivate` _walkingeffect)
      (`self.HandleBeginFalling` (`self.CoyoteTimeDuration`)))))

(event `EnhancedInput|/Game/Blueprints/Input/Actions/IA_NextPowerup`
  (params (ActionValue :type Boolean) (ElapsedSeconds :type "Float (double-precision)") (TriggeredSeconds :type "Float (double-precision)") (InputAction :type "InputAction Object Reference" :default "/Game/Blueprints/Input/Actions/IA_NextPowerup.IA_NextPowerup"))
  (:`Triggered`
    (`KismetSystemLibrary.LogString` "NextPowerup_Event triggered")
    (`self.NextPowerup`)))

(event `Key|Gamepad_DPad_Down` :consume false :overrideparent false
  (params (Key :type "Key Structure"))
  (:`Pressed`
    (`KismetSystemLibrary.LogString` "NextPowerup_Event triggered manual")))

(event `Key|Gamepad_DPad_Up`
  (params (Key :type "Key Structure"))
  (:`Pressed`
    (`KismetSystemLibrary.LogString` "PreviousPowerup_Event triggered manual")))

(event `EnhancedInput|/Game/Blueprints/Input/Actions/IA_Parry`
  (params (ActionValue :type Boolean) (ElapsedSeconds :type "Float (double-precision)") (TriggeredSeconds :type "Float (double-precision)") (InputAction :type "InputAction Object Reference" :default "/Game/Blueprints/Input/Actions/IA_Parry.IA_Parry"))
  (:`Triggered`
    (`self.OnParryActivated`)))

(event `EnhancedInput|/Game/Blueprints/Input/Actions/IA_PreviousPowerup`
  (params (ActionValue :type Boolean) (ElapsedSeconds :type "Float (double-precision)") (TriggeredSeconds :type "Float (double-precision)") (InputAction :type "InputAction Object Reference" :default "/Game/Blueprints/Input/Actions/IA_PreviousPowerup.IA_PreviousPowerup"))
  (:`Triggered`
    (`KismetSystemLibrary.LogString` "PreviousPowerup_Event triggered")
    (`self.PreviousPowerup`)))

(event `EnhancedInput|/Game/Blueprints/Input/Actions/IA_PerfectBounce`
  (params (ActionValue :type Boolean) (ElapsedSeconds :type "Float (double-precision)") (TriggeredSeconds :type "Float (double-precision)") (InputAction :type "InputAction Object Reference" :default "/Game/Blueprints/Input/Actions/IA_PerfectBounce.IA_PerfectBounce"))
  (:`Triggered`
    (`self.OnBounceActivated`)))

(event `EnhancedInput|/Game/Blueprints/Input/Actions/IA_ActivatePowerup`
  (params (ActionValue :type Boolean) (ElapsedSeconds :type "Float (double-precision)") (TriggeredSeconds :type "Float (double-precision)") (InputAction :type "InputAction Object Reference" :default "/Game/Blueprints/Input/Actions/IA_ActivatePowerup.IA_ActivatePowerup"))
  (:`Triggered`
    (`KismetSystemLibrary.LogString` "ActivatePowerup_Event triggered")
    (`self.ActivatePowerup`)))

(event `EnhancedInput|/Game/Blueprints/Input/Actions/Tutorial/IA_TutorialAccept`
  (params (ActionValue :type Boolean) (ElapsedSeconds :type "Float (double-precision)") (TriggeredSeconds :type "Float (double-precision)") (InputAction :type "InputAction Object Reference" :default "/Game/Blueprints/Input/Actions/Tutorial/IA_TutorialAccept.IA_TutorialAccept"))
  (:`Triggered`
    (`self.OnTutorialAccept`)))

(event `self.OnVictory`
  (`|PlayMontage` (`self.Mesh`) "/Game/Assets/Character/Animations/AM_Victory.AM_Victory"))

(event `self.OnDeath`
  (params (DamageInstigator :type "DONPlayerCharacter Object Reference"))
  (`/Game/Blueprints/UI/Common/BFL_UIFunctions.DisplayMessage` self (make `/Game/Blueprints/UI/Common/FHUDMessage` "Player died" (`self.GetPlayerColor`)))
  (`PlayerController.ClientStartCameraShake` :`self` (`GameplayStatics.GetPlayerController` 0) :`Shake` "/Game/Blueprints/CameraShakes/BP_DeathShake.BP_DeathShake_C"))

(event `self.ParryCollider.OnComponentHit`
  (params (HitComponent :type "PrimitiveComponent Object Reference") (OtherActor :type "Actor Object Reference") (OtherComp :type "PrimitiveComponent Object Reference") (NormalImpulse :type "Vector Structure") (Hit :type "HitResult Structure (by ref)"))
  (`GameplayCueFunctionLibrary.ExecuteGameplayCueOnActor` self (struct :`TagName` "GameplayCue.Player.ParrySuccess") (`AbilitySystemBlueprintLibrary.MakeGameplayCueParameters` 0.0)))

(fn `UserConstructionScript`)