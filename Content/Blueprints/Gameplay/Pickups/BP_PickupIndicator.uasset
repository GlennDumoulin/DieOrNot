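; BP_PickupIndicator is a pickup indicator actor that changes its decal glow and fires an effect according to a percentage passed to UpdateVisualization.
; It creates the decal's dynamic material on BeginPlay, or on update if missing.
; Above 90% it raises Strength and activates NSPickupIndicator; below 10% it dims Strength.
; Two DoOnce nodes reset each other, forming a hysteresis latch so each transition fires once.
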(event `self.ReceiveBeginPlay`
  (`/Engine/EditorBlueprintResources/StandardMacros.IsValid` (`self.Material`)
    (:`Is Not Valid`
      (`self.MakeMaterial`))))

(event `MakeMaterial`
  (bind _returnvalue (`DecalComponent.CreateDynamicMaterialInstance` (`self.Decal`)))
  (set `self.Material` _returnvalue))

(event `self.UpdateVisualization`
  (params (percentage :type "Float (single-precision)"))
  (bind _material (`self.Material`))
  (`/Engine/EditorBlueprintResources/StandardMacros.IsValid` _material
    (:`Is Valid`
      _)
    (:`Is Not Valid`
      (`self.MakeMaterial`)))
  (if (> percentage 0.9)
    (`/Engine/EditorBlueprintResources/StandardMacros.DoOnce` false :!label _label
      (:`Completed`
        (`MaterialInstanceDynamic.SetScalarParameterValue` _material "Strength" 5.0)
        (`ActorComponent.Activate` (`self.NS_PickupIndicator`) true)
        (goto _label_2 :!via `Reset`)))
    (elif (< percentage 0.1)
      (`/Engine/EditorBlueprintResources/StandardMacros.DoOnce` false :!label _label_2
        (:`Completed`
          (`MaterialInstanceDynamic.SetScalarParameterValue` _material "Strength" 0.3)
          (goto _label :!via `Reset`))))))

(fn `UserConstructionScript`)