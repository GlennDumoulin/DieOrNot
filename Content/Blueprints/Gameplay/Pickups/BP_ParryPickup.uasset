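; BP_ParryPickup is a pickup child Blueprint that adds spawn telegraph and idle effects, and destroys itself when the gamemode's round ends.
; UpdateProgress uses a resettable DoOnce in the last three seconds of the spawn timer to play Niagara spawn VFX, fade in active audio and play a delayed spawn sound.
; Enable and disable call the parent, then toggle idle Niagara, with disable also fading out audio.
; The overlap handler is empty.
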(event `self.ReceiveBeginPlay`
  (add `/Game/Blueprints/Gameplay/BP_Gamemode.OnRoundEndEvent` (cast `/Game/Blueprints/Gameplay/BP_Gamemode` (`GameplayStatics.GetGameMode`) :!pure true) (delegate `End`)))

(event `End`
  (`self.K2_DestroyActor`))

(event `self.UpdateProgress`
  (params (percentage :type "Float (single-precision)"))
  (if (> 3.0 (- (`self.SpawnTime`) (* percentage (`self.SpawnTime`))))
    (`/Engine/EditorBlueprintResources/StandardMacros.DoOnce` false :!label _label
      (:`Completed`
        (`NiagaraFunctionLibrary.SpawnSystemAtLocation` "/Game/RFX/Systems/NS_PickUp_Spawn.NS_PickUp_Spawn" (`self.K2_GetActorLocation`))
        (`AudioComponent.FadeIn` (`self.ActiveSound`) 1.0 1.0 0.0 "Linear")
        (`KismetSystemLibrary.Delay` 1.5)
        (`GameplayStatics.PlaySoundAtLocation` "/Game/SFX/Game/SW_PickupSpawn.SW_PickupSpawn" (`self.K2_GetActorLocation`) (struct) 0.5 1.0 0.0 null null null null)))
    (else
      (goto _label :!via `Reset`))))

(event `self.SphereCollider.OnComponentBeginOverlap`
  (params (OverlappedComponent :type "PrimitiveComponent Object Reference") (OtherActor :type "Actor Object Reference") (OtherComp :type "PrimitiveComponent Object Reference") (OtherBodyIndex :type Integer) (bFromSweep :type Boolean) (SweepResult :type "HitResult Structure (by ref)")))

(event `self.EnablePickup`
  (`parent.EnablePickup`)
  (`ActorComponent.Activate` (`self.NS_pickUp_Idle`) true))

(event `self.DisablePickup`
  (`parent.DisablePickup`)
  (`ActorComponent.Deactivate` (`self.NS_pickUp_Idle`))
  (`AudioComponent.FadeOut` (`self.ActiveSound`) 1.0 0.0 "Linear"))

(fn `UserConstructionScript`)