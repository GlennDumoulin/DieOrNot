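; Game mode Blueprint that owns the round-based UI flow and notifies the level camera as rounds start and end.
; BeginPlay builds an aspect-limit root widget hosting the HUD and round screens, adds a mouse-handler overlay, finds the camera and optionally spawns a tutorial manager.
; Round and game events show or create the relevant screens, with round transitions also toggling navigation mode.
; A helper switches every player controller's input mode.
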(event `self.ReceiveTick`
  (params (DeltaSeconds :type "Float (single-precision)")))

(event `self.ReceiveBeginPlay`
  (bind _returnvalue (`|CreateWidget` "/Game/Blueprints/UI/Common/WBP_AspectLimit.WBP_AspectLimit_C"))
  (bind _output_get (set `self.Root` _returnvalue))
  (`UserWidget.AddToViewport` _output_get 9)
  (bind _returnvalue_2 (`|CreateWidget` "/Game/Blueprints/UI/Common/WBP_MouseHandler.WBP_MouseHandler_C"))
  (`UserWidget.AddToViewport` _returnvalue_2 50)
  (bind _returnvalue_3 (`|CreateWidget` "/Game/Blueprints/UI/Game/WBP_GameHUD.WBP_GameHUD_C"))
  (bind _output_get_2 (set `self.HUD` _returnvalue_3))
  (`/Game/Blueprints/UI/Common/WBP_AspectLimit.AddChild` (`self.Root`) _output_get_2)
  (`Widget.SetVisibility` _output_get_2 "Hidden")
  (bind _returnvalue_4 (`|CreateWidget` "/Game/Blueprints/UI/Game/WBP_RoundEndScreen.WBP_RoundEndScreen_C"))
  (bind _output_get_3 (set `self.RoundEndScreen` _returnvalue_4))
  (`/Game/Blueprints/UI/Common/WBP_AspectLimit.AddChild` (`self.Root`) _output_get_3)
  (`Widget.SetVisibility` _output_get_3 "Hidden")
  (bind _returnvalue_5 (`GameplayStatics.GetActorOfClass` "/Game/Blueprints/Level/BP_LevelCamera.BP_LevelCamera_C"))
  (set `self.Camera` _returnvalue_5)
  (if (`DONGameInstance.GetEnableTutorials` (cast `DONGameInstance` (`GameplayStatics.GetGameInstance`) :!pure true))
    (`|SpawnActorFromClass` "/Game/Blueprints/Level/BP_TutorialManager.BP_TutorialManager_C" (`KismetMathLibrary.MakeTransform` (0.0 0.0 0.0)) "Undefined" "OverrideRootScale" null null)))

(event `self.OnRoundStart`
  (bind _roundstartscreen (`self.RoundStartScreen`))
  (`self.SwitchNavigationMode` false)
  (`/Engine/EditorBlueprintResources/StandardMacros.IsValid` (`self.RoundStartScreen`)
    (:`Is Valid`
      (`Widget.SetVisibility` _roundstartscreen "SelfHitTestInvisible")
      (`/Game/Blueprints/UI/Game/WBP_RoundStartScreen.HandleTimer` _roundstartscreen))
    (:`Is Not Valid`
      (bind _returnvalue (`|CreateWidget` "/Game/Blueprints/UI/Game/WBP_RoundStartScreen.WBP_RoundStartScreen_C"))
      (bind _output_get (set `self.RoundStartScreen` _returnvalue))
      (`/Game/Blueprints/UI/Common/WBP_AspectLimit.AddChild` (`self.Root`) _output_get)))
  (`Widget.SetVisibility` (`self.HUD`) "SelfHitTestInvisible")
  (`/Game/Blueprints/UI/Game/WBP_GameHUD.RoundStart` (`self.HUD`))
  (`/Game/Blueprints/Level/BP_LevelCamera.RoundStart` (`self.Camera`)))

(event `self.OnRoundEnd`
  (bind _roundendscreen (`self.RoundEndScreen`))
  (`/Engine/EditorBlueprintResources/StandardMacros.IsValid` (`self.RoundEndScreen`)
    (:`Is Valid`
      (`Widget.SetVisibility` _roundendscreen "SelfHitTestInvisible"))
    (:`Is Not Valid`
      (bind _returnvalue (`|CreateWidget` "/Game/Blueprints/UI/Game/WBP_RoundEndScreen.WBP_RoundEndScreen_C"))
      (bind _output_get (set `self.RoundEndScreen` _returnvalue))
      (`/Game/Blueprints/UI/Common/WBP_AspectLimit.AddChild` (`self.Root`) _output_get)))
  (`self.SwitchNavigationMode` true)
  (`/Game/Blueprints/UI/Game/WBP_RoundEndScreen.ShowDetails` _roundendscreen)
  (`/Game/Blueprints/Level/BP_LevelCamera.RoundEnd` (`self.Camera`) self)
  (`self.OnRoundEndEvent`))

(event `self.OnGameEnd`
  (bind _returnvalue (`|CreateWidget` "/Game/Blueprints/UI/Game/WBP_GameEndScreen.WBP_GameEndScreen_C"))
  (`/Game/Blueprints/UI/Common/WBP_AspectLimit.AddChild` (`self.Root`) _returnvalue))

(fn `SetPlayerFocus`
  (params (Value :type Boolean) (InWidgetToFocus :type "Widget Object Reference"))
  (for _index (range (`GameplayStatics.GetNumPlayerControllers`))
    (if Value
      (bind _returnvalue (`GameplayStatics.GetPlayerController` _index))
      (`WidgetBlueprintLibrary.SetInputMode_GameOnly` _returnvalue true)
      (else
        (`WidgetBlueprintLibrary.SetInputMode_GameAndUIEx` _returnvalue InWidgetToFocus "DoNotLock" true true)))))

(fn `UserConstructionScript`)