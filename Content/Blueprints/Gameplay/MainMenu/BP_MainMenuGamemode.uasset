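; Main menu game mode that creates the menu UI and lets one player at a time take control of it.
; BeginPlay nests the main menu inside an aspect-limit widget and adds a mouse handler widget on a higher layer.
; FocusMenu toggles ownership: the claiming player's pawn is frozen through time dilation, loses collision and gets a MenuActive gameplay cue.
; Only that same player can release the menu, which restores the pawn.
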(event `self.ReceiveBeginPlay`
  (bind _returnvalue (`|CreateWidget` "/Game/Blueprints/UI/Common/WBP_AspectLimit.WBP_AspectLimit_C"))
  (`UserWidget.AddToViewport` _returnvalue 0)
  (bind _returnvalue_2 (`|CreateWidget` "/Game/Blueprints/UI/MainMenu/WBP_MainMenu.WBP_MainMenu_C"))
  (`/Game/Blueprints/UI/Common/WBP_AspectLimit.AddChild` _returnvalue _returnvalue_2)
  (set `self.Root` _returnvalue_2)
  (set `self.Menu` _returnvalue_2)
  (bind _returnvalue_3 (`|CreateWidget` "/Game/Blueprints/UI/Common/WBP_MouseHandler.WBP_MouseHandler_C"))
  (`UserWidget.AddToViewport` _returnvalue_3 50))

(event `FocusMenu`
  (params (PlayerController :type "PlayerController Object Reference"))
  (bind _returnvalue (`AbilitySystemBlueprintLibrary.MakeGameplayCueParameters` 0.0))
  (bind _returnvalue_2 (`Controller.K2_GetPawn` PlayerController))
  (bind _menu (`self.Menu`))
  (bind _menuplayer (`self.MenuPlayer`)
    (:`then`
      (if (== _menuplayer PlayerController)
        (`Widget.SetUserFocus` _menu PlayerController)
        (set `self.MenuPlayer` null)
        (set `Actor.CustomTimeDilation` 1.0 _returnvalue_2)
        (`GameplayCueFunctionLibrary.RemoveGameplayCueOnActor` _returnvalue_2 (struct :`TagName` "GameplayCue.Game.MenuActive") _returnvalue)
        (`self.SetActorEnableCollision` _returnvalue_2 true)))
    (:`else`
      (`/Game/Blueprints/UI/Common/WBP_FocusableRoot.SetPlayerFocus` _menu PlayerController null)
      (`/Game/Blueprints/UI/MainMenu/WBP_MainMenu.FocusControlsButton` _menu)
      (set `self.MenuPlayer` PlayerController)
      (set `Actor.CustomTimeDilation` 0.0 _returnvalue_2)
      (`GameplayCueFunctionLibrary.AddGameplayCueOnActor` _returnvalue_2 (struct :`TagName` "GameplayCue.Game.MenuActive") _returnvalue)
      (`self.SetActorEnableCollision` _returnvalue_2 false))))

(fn `UserConstructionScript`)