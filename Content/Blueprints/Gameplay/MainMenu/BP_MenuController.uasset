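; Player controller for the main menu that handles readying up, color changes and menu navigation through Enhanced Input.
; Ready input toggles state through a FlipFlop, ignored for the gamemode's MenuPlayer or while the game is starting.
; Color input cycles the player's color with Niagara and sound effects if the pawn is visible.
; Navigate input asks BP_MainMenuGamemode to focus the menu on this controller, only when ready.
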(event `self.ReceiveBeginPlay`)

(event `EnhancedInput|/Game/Blueprints/Input/Actions/MenuActions/IA_MenuReady`
  (params (ActionValue :type Boolean) (ElapsedSeconds :type "Float (double-precision)") (TriggeredSeconds :type "Float (double-precision)") (InputAction :type "InputAction Object Reference" :default "/Game/Blueprints/Input/Actions/MenuActions/IA_MenuReady.IA_MenuReady"))
  (bind _asbp_main_menu_gamemode (cast `/Game/Blueprints/Gameplay/MainMenu/BP_MainMenuGamemode` (`GameplayStatics.GetGameMode`) :!pure true))
  (:`Triggered`
    (if (not (or (== (`/Game/Blueprints/Gameplay/MainMenu/BP_MainMenuGamemode.MenuPlayer` _asbp_main_menu_gamemode) self) (`/Game/Blueprints/Gameplay/MainMenu/BP_MainMenuGamemode.GameStarting` _asbp_main_menu_gamemode)))
      (bind _isa (`/Engine/EditorBlueprintResources/StandardMacros.FlipFlop`)
        (:`A`
          _)
        (:`B`
          _))
      (`self.SetReady` _isa))))

(event `EnhancedInput|/Game/Blueprints/Input/Actions/MenuActions/IA_MenuNextColor`
  (params (ActionValue :type Boolean) (ElapsedSeconds :type "Float (double-precision)") (TriggeredSeconds :type "Float (double-precision)") (InputAction :type "InputAction Object Reference" :default "/Game/Blueprints/Input/Actions/MenuActions/IA_MenuNextColor.IA_MenuNextColor"))
  (bind _returnvalue (`self.K2_GetPawn`))
  (bind _returnvalue_2 (`self.K2_GetActorLocation` _returnvalue))
  (:`Triggered`
    (if (not (`Actor.bHidden` _returnvalue))
      (`self.NextPlayerColor`)
      (`NiagaraFunctionLibrary.SpawnSystemAtLocation` "/Game/RFX/Systems/NS_Chara_ChangeColor.NS_Chara_ChangeColor" _returnvalue_2)
      (`GameplayStatics.PlaySoundAtLocation` "/Game/SFX/Menu/SW_ColorChange.SW_ColorChange" _returnvalue_2 (struct) 0.2 1.0 0.0 null null null null))))

(event `EnhancedInput|/Game/Blueprints/Input/Actions/MenuActions/IA_MenuNavigate`
  (params (ActionValue :type Boolean) (ElapsedSeconds :type "Float (double-precision)") (TriggeredSeconds :type "Float (double-precision)") (InputAction :type "InputAction Object Reference" :default "/Game/Blueprints/Input/Actions/MenuActions/IA_MenuNavigate.IA_MenuNavigate"))
  (:`Triggered`
    (if (`self.IsReady`)
      (`/Game/Blueprints/Gameplay/MainMenu/BP_MainMenuGamemode.FocusMenu` (cast `/Game/Blueprints/Gameplay/MainMenu/BP_MainMenuGamemode` (`GameplayStatics.GetGameMode`) :!pure true) self))))

(fn `UserConstructionScript`)