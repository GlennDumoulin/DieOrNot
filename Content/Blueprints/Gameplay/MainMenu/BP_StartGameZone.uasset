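; Main menu zone actor that shows status text on a widget and handles the transition into the game, starting with a "Not enough players connected" message.
; Timer start attaches Niagara effects to each player's menu pawn, hidden for hidden pawns, and timer end deactivates them.
; Starting the game disables the menu, flags the game mode as starting, fades to black, clears players and opens the persistent game level.
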(event `self.ReceiveBeginPlay`
  (bind _aswbp_start_game_zone (cast `/Game/Blueprints/UI/MainMenu/WBP_StartGameZone` (`WidgetComponent.GetWidget` (`self.Widget`))))
  (bind _output_get (set `self.WidgetRef` _aswbp_start_game_zone))
  (`TextBlock.SetText` (`/Game/Blueprints/UI/MainMenu/WBP_StartGameZone.Text` _output_get) "Not enough players connected"))

(event `self.HandleStartGame`
  (bind _fadeduration (`self.FadeDuration`))
  (bind _asbp_main_menu_gamemode (cast `/Game/Blueprints/Gameplay/MainMenu/BP_MainMenuGamemode` (`GameplayStatics.GetGameMode`) :!pure true))
  (`/Game/Blueprints/UI/MainMenu/WBP_MainMenu.Disable` (`/Game/Blueprints/Gameplay/MainMenu/BP_MainMenuGamemode.Menu` _asbp_main_menu_gamemode))
  (set `/Game/Blueprints/Gameplay/MainMenu/BP_MainMenuGamemode.GameStarting` true _asbp_main_menu_gamemode)
  (`DONFunctionLibrary.FadeScreen` _fadeduration true)
  (`KismetSystemLibrary.Delay` _fadeduration)
  (`MenuGameMode.ClearPlayers` _asbp_main_menu_gamemode)
  (`GameplayStatics.OpenLevelBySoftObjectPtr` "/Game/Maps/PersistentGame.PersistentGame"))

(event `self.OnTimerStart`
  (for _array_element (`GameStateBase.PlayerArray` (`GameplayStatics.GetGameState`))
    (bind _asbp_menu_player (cast `/Game/Blueprints/Gameplay/MainMenu/BP_MenuPlayer` (`PlayerState.GetPawn` _array_element)))
    (bind _returnvalue (`NiagaraFunctionLibrary.SpawnSystemAttached` "/Game/RFX/Systems/NS_PickUp_Spawn2.NS_PickUp_Spawn2" (`Actor.RootComponent` _asbp_menu_player) "None" (0.0 0.0 0.0) (struct) "KeepRelativeOffset" true))
    (if (`Actor.bHidden` _asbp_menu_player)
      (`SceneComponent.SetHiddenInGame` _returnvalue true false))
    (`KismetArrayLibrary.Array_Add` (`self.ParticleSystems`) _returnvalue)))

(event `self.OnTimerEnd`
  (bind _particlesystems (`self.ParticleSystems`))
  (for _array_element _particlesystems
    (`/Engine/EditorBlueprintResources/StandardMacros.IsValid` _array_element
      (:`Is Valid`
        (`ActorComponent.Deactivate` _array_element))))
  (`KismetArrayLibrary.Array_Clear` _particlesystems))

(event `self.SetText`
  (params (NewText :type String))
  (bind _widgetref (`self.WidgetRef`))
  (`/Engine/EditorBlueprintResources/StandardMacros.IsValid` _widgetref
    (:`Is Valid`
      (`TextBlock.SetText` (`/Game/Blueprints/UI/MainMenu/WBP_StartGameZone.Text` _widgetref) (`KismetTextLibrary.Conv_StringToText` NewText)))))

(fn `UserConstructionScript`)