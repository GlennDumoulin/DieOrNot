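; Player death effect that shatters a Chaos fracture and adds a splatter burst and decal-like plane, tinted with the player's color.
; BeginPlay spawns a temporary FS_MasterField, scales its radial force from bullet velocity or a fallback, triggers it, then destroys it.
; The Niagara splatter faces along the offset from fracture to hit location, while a timeline grows the randomly textured, randomly rotated plane.
; Collision sound logic is present but unconnected.
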(event `self.ReceiveBeginPlay`
  (bind _player (`self.Player`))
  (bind _bullet (`self.Bullet`))
  (bind _plane (`self.Plane`))
  (bind _playercolor (`DONPlayerCharacter.PlayerColor` _player))
  (`/Engine/EditorBlueprintResources/StandardMacros.IsValid` _player
    (:`Is Valid`
      (for (_array_element _array_index) (`MeshComponent.GetMaterials` (`self.Fracture`))
        (bind _returnvalue (`PrimitiveComponent.CreateDynamicMaterialInstance` (`self.Fracture`) _array_index _array_element "None"))
        (`/Engine/EditorBlueprintResources/StandardMacros.IsValid` _returnvalue
          (:`Is Valid`
            (`MaterialInstanceDynamic.SetVectorParameterValue` _returnvalue "Color" _playercolor))))
      (bind _returnvalue_2 (`PrimitiveComponent.CreateDynamicMaterialInstance` (`self.Plane`) 0 "/Game/Materials/Decals/M_DeathSplatter.M_DeathSplatter" "None"))
      (`MaterialInstanceDynamic.SetVectorParameterValue` _returnvalue_2 "Color" _playercolor)
      (`MaterialInstanceDynamic.SetTextureParameterValue` _returnvalue_2 "Tex" (select `int` (`KismetMathLibrary.RandomIntegerInRange` 0 2) :`0` "/Game/Textures/Decals/T_BloodSplatter_Temp_01.T_BloodSplatter_Temp_01" :`1` "/Game/Textures/Decals/T_BloodSplatter_Temp_02.T_BloodSplatter_Temp_02" :`2` "/Game/Textures/Decals/T_BloodSplatter_Temp_03.T_BloodSplatter_Temp_03" :!type "Texture Object Reference"))
      (set `self.Material` _returnvalue_2))
    (:`Is Not Valid`
      _))
  (bind _returnvalue_3 (`|SpawnActorFromClass` "/Engine/EditorResources/FieldNodes/FS_MasterField.FS_MasterField_C" (`KismetMathLibrary.MakeTransform` (`self.Location`)) "AlwaysSpawn" "OverrideRootScale" null null))
  (set `/Engine/EditorResources/FieldNodes/FS_MasterField.ActivationType` "NewEnumerator4" _returnvalue_3)
  (`|ExecutionSequence`
    (:`then_0`
      (`/Engine/EditorBlueprintResources/StandardMacros.IsValid` _bullet
        (:`Is Valid`
          (set `/Engine/EditorResources/FieldNodes/FS_MasterField.Radial Magnitude` (* (`KismetMathLibrary.VSize` (`self.GetVelocity` _bullet)) 1.5) _returnvalue_3))
        (:`Is Not Valid`
          (set `/Engine/EditorResources/FieldNodes/FS_MasterField.Radial Magnitude` 500.0 _returnvalue_3))))
    (:`then_1`
      (`NiagaraComponent.SetVariableLinearColor` (`self.Splatter`) "Color" _playercolor)
      (`SceneComponent.K2_SetWorldRotation` (`self.Splatter`) (`KismetMathLibrary.Conv_VectorToRotator` (- (`self.Location`) (`SceneComponent.K2_GetComponentLocation` (`self.Fracture`)))) false false)
      (`ActorComponent.Activate` (`self.Splatter`) true))
    (:`then_2`
      (`/Engine/EditorResources/FieldNodes/FS_MasterField.CE_Trigger` _returnvalue_3)
      (`KismetSystemLibrary.Delay` 1.0)
      (`self.K2_DestroyActor` _returnvalue_3))
    (:`then_3`
      (`SceneComponent.K2_SetWorldRotation` _plane (`KismetMathLibrary.MakeRotator` 90.0 (`KismetMathLibrary.RandomFloatInRange` 0.0 360.0) 90.0) false false)
      (`SceneComponent.K2_AddWorldOffset` _plane (-100.0 0.0 0.0) false false))
    (:`then_4`
      (bind (_direction _newtrack_0) (`Timeline|Timeline` :!via `PlayFromStart`)
        (:`Update`
          (`SceneComponent.SetWorldScale3D` (`self.Plane`) (`KismetMathLibrary.Conv_DoubleToVector` (* _newtrack_0 4.5))))))))

(event `CustomEvent`
  (params (CollisionInfo :type "ChaosPhysicsCollisionInfo Structure (by ref)"))
  (if (!= CollisionInfo_OtherComponent CollisionInfo_Component)
    _))

(fn `UserConstructionScript`)