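; Player-owned projectile whose Niagara trail and prediction effects take the owning player's color.
; On BeginPlay it applies that color, then enables actor collision one tick later.
; OnDestroyBullet disables tick and collision and hides the mesh and prediction visuals, then a tick later stops movement and spawns the NS_ShootAgain effect in place.
; Hit and overlap events are empty, and this graph never calls DestroyActor.
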(event `self.ReceiveBeginPlay`
  ;[0 0 0] Set the RFX colors
  (`FXSystemComponent.SetColorParameter` (`self.NS_BulletTrail`) "OwnerColor" (`DONPlayerCharacter.GetPlayerColor` (`self.PlayerOwner`)))
  (`FXSystemComponent.SetColorParameter` (`self.NS_BulletPrediction`) "OwnerColor" (`DONPlayerCharacter.GetPlayerColor` (`self.PlayerOwner`)))
  (`KismetSystemLibrary.DelayUntilNextTick`)
  (`self.SetActorEnableCollision` true))

(event `self.SphereCollider.OnComponentHit`
  (params (HitComponent :type "PrimitiveComponent Object Reference") (OtherActor :type "Actor Object Reference") (OtherComp :type "PrimitiveComponent Object Reference") (NormalImpulse :type "Vector Structure") (Hit :type "HitResult Structure (by ref)")))

(event `self.OnDestroyBullet`
  (`self.SetActorTickEnabled` false)
  (`self.SetActorEnableCollision` false)
  (`SceneComponent.SetHiddenInGame` (`self.Mesh`) true false)
  (`SceneComponent.SetHiddenInGame` (`self.NS_BulletPrediction`) true false)
  (`SceneComponent.SetHiddenInGame` (`self.PredictionRoot`) true false)
  (`KismetSystemLibrary.DelayUntilNextTick`)
  (`MovementComponent.StopMovementImmediately` (`self.ProjectileMovement`))
  (`NiagaraFunctionLibrary.SpawnSystemAtLocation` "/Game/RFX/Systems/NS_ShootAgain.NS_ShootAgain" (`self.K2_GetActorLocation`)))

(fn `UserConstructionScript`)